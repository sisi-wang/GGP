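; BP_EnemyBase is an enemy base Blueprint that passes perception of the player to its AI controller.
; On a perception update for player pawn 0, it casts its controller to BPAIC_Enemy and writes the blackboard's player_ref key.
; The key holds the player pawn while sensed and is cleared otherwise.
; Debug prints show the sensed state or a failed cast.
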(event OnTargetPerceptionUpdated(AIPerception)
  (params (Actor :type Actor%20Object%20Reference) (Stimulus :type AI%20Stimulus%20Structure))
  (bind _bsuccessfullysensed (Utilities|Struct|BreakAIStimulus Stimulus))
  ;[0.15 0.15 0.15 0.5] On perceive player character
  (if (== (Game|Player|GetPlayerPawn 0) Actor)
    (bind _asbpaic_enemy (Utilities|Casting|CastToBPAIC_Enemy (Pawn|GetController))
      (:then
        (AI|Components|Blackboard|SetValueasObject (AI|GetBlackboard _asbpaic_enemy) (Utilities|Name|MakeLiteralName "player_ref") (Utilities|SelectObject (Game|Player|GetPlayerPawn 0) 0 _bsuccessfullysensed))
        (Development|PrintString (Utilities|String|ToString(Boolean) _bsuccessfullysensed)))
      (:CastFailed
        (Development|PrintString "Hello")))))

(event EventBeginPlay)

(event Collision|EventActorBeginOverlap
  (params (OtherActor :type Actor%20Object%20Reference)))

(fn ConstructionScript)