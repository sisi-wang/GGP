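; BP_EnemyBrushBox is a placeable trigger box that spawns one enemy when the player enters it.
; On overlap by player pawn 0, it spawns EnemyClass at the actor-relative SpawnLocation, facing the actor's yaw, and stores it in SpawnedPawn.
; An IsSpawned flag blocks repeat spawns, and an invalid class prints an error.
; ShowDebugDraw toggles in-game visibility of the box and arrow at BeginPlay.
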(event OnComponentBeginOverlap(Box)
  (params (OverlappedComponent :type Primitive%20Component%20Object%20Reference) (OtherActor :type Actor%20Object%20Reference) (OtherComp :type Primitive%20Component%20Object%20Reference) (OtherBodyIndex :type Integer) (bFromSweep :type Boolean) (SweepResult :type Hit%20Result%20Structure%20%28by%20ref%29))
  (bind _returnvalue (Transformation|GetActorTransform))
  ;[0.15 0.15 0.15 0.5] Spawn the enemy actor when player enter
  (if (Utilities|IsValidClass (Variables|Default|Getenemy_class))
    (if (and (== OtherActor (Game|Player|GetPlayerPawn 0)) (not (Variables|Default|Getis_spawned)))
      (bind _returnvalue_2 (Game|SpawnActorfromClass (Variables|Default|Getenemy_class) (Math|Transform|MakeTransform (Math|Transform|TransformLocation _returnvalue (Variables|Default|Getspawn_location)) (Math|Rotator|MakeRotator 0.0 0.0 (.Yaw (Math|Rotator|BreakRotator (.Rotation (Math|Transform|BreakTransform _returnvalue)))))) "Undefined" "MultiplyWithRoot" 0 0))
      (Variables|Default|Setspawned_pawn _returnvalue_2)
      (Variables|Default|Setis_spawned true))
    (else
      (Development|PrintString "Spawn enemy failed, the class of enemy is invalid." true true "(R=1.000000,G=0.034909,B=0.000000,A=1.000000)" 1e+01))))

(event EventBeginPlay
  (Development|SetHiddeninGame (Variables|Default|GetBox) (not (Variables|Default|Getshow_debug_draw)) false))

(event Collision|EventActorBeginOverlap
  (params (OtherActor :type Actor%20Object%20Reference)))

(event EventTick
  (params (DeltaSeconds :type Float%20%28single-precision%29)))

(fn ConstructionScript)