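; BP_CaptionsTrigger is a box trigger that shows captions and task text when the player pawn overlaps it.
; It finds an existing BP_CaptionsDisplay actor or spawns one, caches it and passes it the text, sound, duration and close-task setting through SetText.
; An IsTriggered flag limits it to one successful activation unless CanRetrigger is set.
; If spawning fails, it prints an error string.
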(event OnComponentBeginOverlap(Box)
  (params (OverlappedComponent :type Primitive%20Component%20Object%20Reference) (OtherActor :type Actor%20Object%20Reference) (OtherComp :type Primitive%20Component%20Object%20Reference) (OtherBodyIndex :type Integer) (bFromSweep :type Boolean) (SweepResult :type Hit%20Result%20Structure%20%28by%20ref%29))
  (if (== OtherActor (Game|Player|GetPlayerPawn 0))
    (CallFunction|TryOpenCaptions)))

(event Custom|TryOpenCaptions
  (if (or (not (Variables|Default|Getis_triggered)) (Variables|Default|Getcan_retrigger))
    (bind _returnvalue (Actor|GetActorOfClass "/Game/Blueprints/Captions/BP_CaptionsDisplay.BP_CaptionsDisplay_C"))
    (Utilities|IsValid _returnvalue
      (:Is%20Valid
        (Variables|Default|Setcap_actor_cache _returnvalue)
        (Default|SetText (Variables|Default|Getcap_actor_cache) (Variables|Default|Getcaptions_text) (Variables|Default|Gettask_text) (Variables|Default|Getclose_task) (Variables|Default|Getcaptions_sound) (Variables|Default|Getcaptions_duration) :!label _label)
        (Variables|Default|Setis_triggered true))
      (:Is%20Not%20Valid
        (bind _returnvalue_2 (Game|SpawnActorfromClass "/Game/Blueprints/Captions/BP_CaptionsDisplay.BP_CaptionsDisplay_C" (Math|Transform|MakeTransform "0, 0, 0" "0, 0, 0" "1.000000,1.000000,1.000000") "AlwaysSpawn" "MultiplyWithRoot" 0 0))
        (bind _output_get (Variables|Default|Setcap_actor_cache _returnvalue_2))
        (Utilities|IsValid _output_get
          (:Is%20Valid
            (goto _label))
          (:Is%20Not%20Valid
            (Development|PrintString "创建失败！")))))))

(event EventBeginPlay)

(event Collision|EventActorBeginOverlap
  (params (OtherActor :type Actor%20Object%20Reference)))

(event EventTick
  (params (DeltaSeconds :type Float%20%28single-precision%29)))

(fn ConstructionScript)