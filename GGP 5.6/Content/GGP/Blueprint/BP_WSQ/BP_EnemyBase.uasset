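; Base enemy character Blueprint that detects the player, handles its own death and pays out money when killed.
; AI perception updates set or clear the player_ref blackboard key on BPAIC_Enemy according to sensing success.
; Death stops movement and sight, unpossesses the controller, flags ABP_Manny as dead, credits BP_Instance with MoneyAdd, then destroys the actor after a delay.
; Tick draws debug health text above the capsule.
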(event OnTargetPerceptionUpdated(AIPerception)
  (params (Actor :type Actor%20Object%20Reference) (Stimulus :type AI%20Stimulus%20Structure))
  (bind _bsuccessfullysensed (Utilities|Struct|BreakAIStimulus Stimulus))
  ;[0.15 0.15 0.15 0.5] On perceive player character
  (if (== (Game|Player|GetPlayerPawn 0) Actor)
    (bind _asbpaic_enemy (Utilities|Casting|CastToBPAIC_Enemy (Pawn|GetController))
      (:then
        (AI|Components|Blackboard|SetValueasObject (AI|GetBlackboard _asbpaic_enemy) (Utilities|Name|MakeLiteralName "player_ref") (Utilities|SelectObject (Game|Player|GetPlayerPawn 0) 0 _bsuccessfullysensed))
        (Development|PrintString (Utilities|String|ToString(Boolean) _bsuccessfullysensed)))
      (:CastFailed
        (Development|PrintString "Hello")))))

(event EventBeginPlay
  (|CallParentFunction))

(event EventHandleDeath
  ;[0.15 0.15 0.15 0.5] Implementation death handle event
  (if (not (Variables|Default|Getis_dead))
    ;;[0.15 0.15 0.15 0.5] Stop all behavior for AI
    (Components|Movement|StopMovementImmediately (Variables|Character|GetCharacterMovement))
    (Class|AIPerceptionComponent|SetSenseEnabled (Variables|Default|GetAIPerception) "/Script/AIModule.AISense_Sight" false)
    (Pawn|UnPossess (Pawn|GetController))
    (bind _asabp_manny (Utilities|Casting|CastToABP_Manny (Components|SkeletalMesh|GetAnimInstance (Variables|Character|GetMesh)))
      (:then
        (Variables|/Game/Characters/Mannequins/Animations/ABP_Manny.ABP_Manny_C|Setis_dead _asabp_manny true))
      (:CastFailed
        _))
    (bind _asbp_instance (Utilities|Casting|CastToBP_Instance (Game|GetGameInstance))
      (:then
        (Default|IncreaseMoney _asbp_instance (Variables|Default|Getmoney_add)))
      (:CastFailed
        _))
    (|CallParentFunction)
    ;;[0.15 0.15 0.15 0.5] delay destroy
    (Utilities|FlowControl|Delay 5.0)
    (Actor|DestroyActor)))

(event EventTick
  (params (DeltaSeconds :type Float%20%28single-precision%29))
  (|CallParentFunction DeltaSeconds)
  (CallFunction|DebugAttribute))

(fn ConstructionScript)

(fn DebugAttribute
  (Rendering|Debug|DrawDebugString (+ (Transformation|GetActorLocation) (Math|Vector|MakeVector 0.0 0.0 (+ (Components|Capsule|GetScaledCapsuleHalfHeight (Variables|Default|GetCapsuleComponent)) 1e+01))) (Utilities|String|Append "health : " (Utilities|String|ToString(Integer) (Math|Float|Truncate (Variables|Default|Gethp))) "/" (Utilities|String|ToString(Integer) (Math|Float|Truncate (Variables|Default|GetMaxhp)))) 0 "(R=1.000000,G=1.000000,B=1.000000,A=1.000000)"))