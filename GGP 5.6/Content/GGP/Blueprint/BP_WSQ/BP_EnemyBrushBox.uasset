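; Trigger-box enemy spawner that runs a looping timer while the player pawn is inside it.
; Each spawn attempt is capped by a live-enemy count, which drops when a spawned enemy's death event fires.
; Spawn transforms use a random box-relative spawn point with random yaw, or a random spot on the box's horizontal plane facing box yaw if none exist.
; Construction applies the box extent, and a debug flag shows the box and arrow.
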(event OnComponentBeginOverlap(Box)
  (params (OverlappedComponent :type Primitive%20Component%20Object%20Reference) (OtherActor :type Actor%20Object%20Reference) (OtherComp :type Primitive%20Component%20Object%20Reference) (OtherBodyIndex :type Integer) (bFromSweep :type Boolean) (SweepResult :type Hit%20Result%20Structure%20%28by%20ref%29))
  ;[0.15 0.15 0.15 0.5] Spawn the enemy actor when player enter
  (if (Utilities|IsValidClass (Variables|Default|Getenemy_class))
    (if (== OtherActor (Game|Player|GetPlayerPawn 0))
      (CallFunction|BeginSpawn))
    (else
      (Development|PrintString "Spawn enemy failed, the class of enemy is invalid." true true "(R=1.000000,G=0.034909,B=0.000000,A=1.000000)" 1e+01))))

(event OnComponentEndOverlap(Box)
  (params (OverlappedComponent :type Primitive%20Component%20Object%20Reference) (OtherActor :type Actor%20Object%20Reference) (OtherComp :type Primitive%20Component%20Object%20Reference) (OtherBodyIndex :type Integer))
  ;[0.15 0.15 0.15 0.5] Spawn the enemy actor when player enter
  (if (== OtherActor (Game|Player|GetPlayerPawn 0))
    (CallFunction|StopSpawn)))

(event Custom|StopSpawn
  ;[0.15 0.15 0.15 0.5] Start and stop spawn
  (Utilities|Time|ClearandInvalidateTimerbyHandle (Variables|Default|Getspawning_timer))
  (Development|PrintString "enemy spawning has stopped." true true "(R=0.447579,G=0.447579,B=0.447579,A=1.000000)" 5.0))

(event Custom|BeginSpawn
  ;[0.15 0.15 0.15 0.5] Start and stop spawn
  (bind _returnvalue (Utilities|Time|SetTimerbyEvent (EventDispatchers|CreateEvent :!event Custom|Spawning) 1.0 true))
  (Variables|Default|Setspawning_timer _returnvalue)
  (Development|PrintString "enemy spawning has started." true true "(R=0.089038,G=0.535497,B=0.272262,A=1.000000)" 5.0))

(event Custom|Spawning
  ;[0.15 0.15 0.15 0.5] Spawning
  (if (< (Variables|Default|Getspawned_enemy) (Variables|Default|Getmax_enemy_count))
    (bind _returnvalue (Game|SpawnActorfromClass (Variables|Default|Getenemy_class) (CallFunction|MakeSpawnTransform) "Undefined" "MultiplyWithRoot" 0 0))
    (Utilities|IsValid _returnvalue
      (:Is%20Valid
        (Math|Integer|IncrementInt (Variables|Default|Getspawned_enemy)
          (:%20%20
            (EventDispatchers|BindEventtoOnDeath _returnvalue (delegate Custom|OnEnemyDeath))))))))

(event Custom|OnEnemyDeath
  ;[0.15 0.15 0.15 0.5] Spawning
  (Math|Integer|DecrementInt (Variables|Default|Getspawned_enemy)))

(event EventBeginPlay
  (Development|SetHiddeninGame (Variables|Default|GetBox) (not (Variables|Default|Getshow_debug_draw)) false))

(event Collision|EventActorBeginOverlap
  (params (OtherActor :type Actor%20Object%20Reference)))

(event EventTick
  (params (DeltaSeconds :type Float%20%28single-precision%29)))

(fn ConstructionScript
  (Components|Box|SetBoxExtent (Variables|Default|GetBox) (Variables|Default|Getbox_extent) true))

(fn MakeSpawnTransform
  (bind _spawn_points (Variables|Default|Getspawn_points))
  (bind _box (Variables|Default|GetBox))
  (bind _returnvalue (Transformation|GetWorldTransform _box))
  (bind _returnvalue_2 (Components|Box|GetScaledBoxExtent _box))
  (bind (_x _y) (Math|Vector|BreakVector _returnvalue_2))
  (bind (_location _rotation) (Math|Transform|BreakTransform _returnvalue))
  (if (> (Utilities|Array|Length _spawn_points) 0)
    (return (Math|Transform|MakeTransform (Math|Transform|TransformLocation _returnvalue (.OutItem (Utilities|Array|Random _spawn_points))) (Math|Rotator|MakeRotator 0.0 0.0 (Math|Random|RandomFloatinRange 0.0 3.6e+02))))
    (else
      (return (Math|Transform|MakeTransform (+ (Math|Vector|RotateVector (Math|Vector|MakeVector (Math|Random|RandomFloatinRange (* _x -1.0) _x) (Math|Random|RandomFloatinRange (* _y -1.0) _y) 0.0) _rotation) _location) (Math|Rotator|MakeRotator 0.0 0.0 (.Yaw (Math|Rotator|BreakRotator _rotation))))))))