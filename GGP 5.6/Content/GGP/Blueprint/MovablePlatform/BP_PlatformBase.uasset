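; Base Blueprint for a movable platform or door that slides or rotates between a closed and a target state.
; TryGotoTarget and TryGoBack check CanGotoTarget and CanBack, which default to true, then flip IsInTarget and enable tick.
; Tick advances OpenFactor over OpenDuration, driving DoorRoot's relative transform, then disables itself and fires fully opened or closed dispatchers.
; The construction script snaps the door to its initial state.
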(event Custom|TryGoBack
  ;[0.15 0.15 0.15 0.5] Try open or close the door
  (if (and (CallFunction|CanBack) (Variables|Default|Getis_in_target))
    (Variables|Default|Setis_in_target false)
    (Actor|Tick|SetActorTickEnabled true)))

(event Custom|TryGotoTarget
  ;[0.15 0.15 0.15 0.5] Try open or close the door
  (if (and (CallFunction|CanGotoTarget) (not (Variables|Default|Getis_in_target)))
    (Variables|Default|Setis_in_target true)
    (Actor|Tick|SetActorTickEnabled true)))

(event Custom|UpdateDoorState
  (bind _door_root (Variables|Default|Getdoor_root))
  (bind _open_factor (Variables|Default|Getopen_factor))
  (bind _tar_open_value (Variables|Default|Gettar_open_value))
  (bind _flip_direction (Variables|Default|Getflip_direction))
  (bind _returnvalue (Math|Conversions|ToFloat(Boolean) _flip_direction))
  (bind _returnvalue_2 (* _returnvalue 2.0))
  (bind _returnvalue_3 (- _returnvalue_2 1.0))
  (bind _returnvalue_4 (* _open_factor _returnvalue_3))
  (bind _returnvalue_5 (* _returnvalue_4 _tar_open_value))
  (bind (_x _y _z) (Math|Vector|BreakVector _returnvalue_5))
  ;[0.15 0.15 0.15 0.5] Set the door opening degree directly
  (if (Variables|Default|Getis_rotation_platform)
    (Transformation|SetRelativeRotation _door_root (Math|Rotator|MakeRotator _x _y _z) false false)
    (else
      (Transformation|SetRelativeLocation _door_root _returnvalue_5 false false))))

(event EventBeginPlay)

(event EventTick
  (params (DeltaSeconds :type Float%20%28single-precision%29))
  ;[0.15 0.15 0.15 0.5] Update door open or close
  (Variables|Default|Setopen_factor (Math|Float|Clamp(Float) (+ (* (/ 1.0 (Variables|Default|Getopen_duration)) DeltaSeconds (- (* (Math|Conversions|ToFloat(Boolean) (Variables|Default|Getis_in_target)) 2.0) 1.0)) (Variables|Default|Getopen_factor))))
  (CallFunction|UpdateDoorState)
  (if (== (Variables|Default|Getopen_factor) (Math|Conversions|ToFloat(Boolean) (Variables|Default|Getis_in_target)))
    (Actor|Tick|SetActorTickEnabled false)
    (if (Variables|Default|Getis_in_target)
      (Default|CallOnFullyOpened)
      (else
        (Default|CallOnFullyClosed)))))

(fn ConstructionScript
  (Variables|Default|Setopen_factor (Math|Conversions|ToFloat(Boolean) (Variables|Default|Getis_in_target)))
  (CallFunction|UpdateDoorState))

(fn GetDoorState
  (bind _door_root (Variables|Default|Getdoor_root))
  (bind _relativerotation (Variables|/Script/Engine.SceneComponent|GetRelativeRotation _door_root))
  (bind (_roll _pitch _yaw) (Math|Rotator|BreakRotator _relativerotation))
  (return (Math|Vector|SelectVector (Math|Vector|MakeVector _roll _pitch _yaw) (Variables|/Script/Engine.SceneComponent|GetRelativeLocation _door_root) (Variables|Default|Getis_rotation_platform))))

(fn CanGotoTarget
  (return true))

(fn CanBack
  (return true))