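; An elevator movable platform that stays locked until enough keys are added, then responds to the player.
; Each AddKey event decrements ActivationRequire, and the CanGotoTarget and CanBack functions allow movement only once it reaches zero or below.
; The player pawn entering the Box trigger calls TryGotoTarget and leaving it calls TryGoBack, with the movement logic defined outside this graph.
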(event OnComponentEndOverlap(Box)
  (params (OverlappedComponent :type Primitive%20Component%20Object%20Reference) (OtherActor :type Actor%20Object%20Reference) (OtherComp :type Primitive%20Component%20Object%20Reference) (OtherBodyIndex :type Integer))
  ;[0.15 0.15 0.15 0.5] Goto target or go back
  (if (== (Game|Player|GetPlayerPawn 0) OtherActor)
    (CallFunction|TryGoBack)))

(event OnComponentBeginOverlap(Box)
  (params (OverlappedComponent :type Primitive%20Component%20Object%20Reference) (OtherActor :type Actor%20Object%20Reference) (OtherComp :type Primitive%20Component%20Object%20Reference) (OtherBodyIndex :type Integer) (bFromSweep :type Boolean) (SweepResult :type Hit%20Result%20Structure%20%28by%20ref%29))
  ;[0.15 0.15 0.15 0.5] Goto target or go back
  (if (== OtherActor (Game|Player|GetPlayerPawn 0))
    (CallFunction|TryGotoTarget)))

(event Custom|AddKey
  ;[0.15 0.15 0.15 0.5] Add a key
  (Math|Integer|DecrementInt (Variables|Default|Getactivation_require)))

(event EventBeginPlay
  (|CallParentFunction) ; 此节点被禁用，将不会被调用。\n从引脚连出引线来编译功能。
)

(event EventTick
  (params (DeltaSeconds :type Float%20%28single-precision%29))
  (|CallParentFunction DeltaSeconds) ; 此节点被禁用，将不会被调用。\n从引脚连出引线来编译功能。
)

(fn ConstructionScript
  (|CallParentFunction))

(fn CanGotoTarget
  (return (<= (Variables|Default|Getactivation_require) 0)))

(fn CanBack
  (return (<= (Variables|Default|Getactivation_require) 0)))