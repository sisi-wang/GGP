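; BP_Instance holds player stats, money and upgrade card pools, apparently as the game instance.
; Setter events copy its max HP, speed, damage and fire rate onto the player pawn, refreshing HP and speed through BP_PLAYER.
; IncreaseMoney adds only non-negative amounts to the balance.
; A card setup event loads every data table row into the upgrade array, then builds a shuffled array of level-one cards.
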(event Custom|Set%20PlayerHP
  (bind _asbp_player (Utilities|Casting|CastToBP_PLAYER (Game|Player|GetPlayerPawn 0)))
  (Variables|/Game/GGP/Blueprint/BP_CharBase.BP_CharBase_C|SetMaxhp _asbp_player (Variables|Default|GetMaxHP))
  (Default|RemakeHP _asbp_player))

(event Custom|Set%20Player%20Speed
  (bind _asbp_player (Utilities|Casting|CastToBP_PLAYER (Game|Player|GetPlayerPawn 0)))
  (Variables|/Script/Engine.CharacterMovementComponent|SetMaxWalkSpeed (Variables|/Script/Engine.Character|GetCharacterMovement _asbp_player) (Variables|Default|GetSpeed))
  (Default|RemakeSpeed _asbp_player))

(event Custom|Set%20player%20Damage
  (bind _asbp_player (Utilities|Casting|CastToBP_PLAYER (Game|Player|GetPlayerPawn 0)))
  (Variables|/Game/GGP/Blueprint/BP_WST/BP_PLAYER.BP_PLAYER_C|SetDamage _asbp_player (Variables|Default|GetDamage)))

(event Custom|Set%20player%20fire%20rate
  (bind _asbp_player (Utilities|Casting|CastToBP_PLAYER (Game|Player|GetPlayerPawn 0)))
  (Variables|/Game/GGP/Blueprint/BP_WST/BP_PLAYER.BP_PLAYER_C|Setfire%20rate _asbp_player (Variables|Default|Getfire%20rate)))

(event Custom|IncreaseMoney
  (params (new_value :type Float%20%28double-precision%29))
  ;[0.15 0.15 0.15 0.5] Increase money for player
  (Variables|Default|Setmoney (+ (Math|Float|Max(Float) new_value 0.0) (Variables|Default|Getmoney))))

(event Custom|add%20card%20arry
  (bind _data_table (Variables|Default|GetData%20Table))
  (bind _outrownames (DataTable|GetDataTableRowNames _data_table))
  (for _array_element _outrownames
    (bind _returnvalue (Utilities|GetDataTableRow _data_table _array_element)
      (:then
        (Utilities|Array|Add (Variables|Default|GetUpgrade%20Card%20Arry) _returnvalue))))
  (bind _outrownames_2 (DataTable|GetDataTableRowNames (Variables|Default|GetData%20Table)))
  (for _array_element_2 _outrownames_2
    (bind _returnvalue_2 (Utilities|GetDataTableRow _data_table _array_element_2)
      (:then
        (if (== (.LVnumber (Utilities|Struct|BreakBP_DATA _returnvalue_2)) 1.0)
          (Utilities|Array|Add (Variables|Default|Getshuffle%20card%20arry) _returnvalue_2)))))
  (Variables|Default|Setshuffle%20card%20arry (Variables|Default|Getshuffle%20card%20arry))
  (Utilities|Array|Shuffle (Variables|Default|Getshuffle%20card%20arry)))