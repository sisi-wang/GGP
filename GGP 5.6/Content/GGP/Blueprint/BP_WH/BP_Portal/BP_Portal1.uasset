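; BP_Portal1 is a portal actor that carries the player character to a destination point when they enter its sphere.
; On overlap by BP_ThirdPersonCharacter, it stores the character's location and Anchor1's location as start and end points, each slightly raised.
; A timeline, triggered with Play rather than PlayFromStart, lerps the character between them using unswept SetActorLocation, so movement is gradual and ignores blocking collision.
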(event OnComponentBeginOverlap(Sphere)
  (params (OverlappedComponent :type Primitive%20Component%20Object%20Reference) (OtherActor :type Actor%20Object%20Reference) (OtherComp :type Primitive%20Component%20Object%20Reference) (OtherBodyIndex :type Integer) (bFromSweep :type Boolean) (SweepResult :type Hit%20Result%20Structure%20%28by%20ref%29))
  (bind _asbp_third_person_character (Utilities|Casting|CastToBP_ThirdPersonCharacter OtherActor))
  (Variables|Default|SetAs%20BP%20Third%20Person%20Character _asbp_third_person_character)
  (Variables|Default|SetPortal_Start (+ (Transformation|GetActorLocation (Variables|Default|GetAs%20BP%20Third%20Person%20Character)) "0.000000,0.000000,30.000000"))
  (Variables|Default|SetPortal_End (+ (Transformation|GetWorldLocation (Variables|Default|GetAnchor1)) "0.000000,0.000000,50.000000"))
  (bind _新建轨道_0 (Timeline|时间轴 Play)
    (:Update
      (Transformation|SetActorLocation (Variables|Default|GetAs%20BP%20Third%20Person%20Character) (Math|Vector|Lerp(Vector) (Variables|Default|GetPortal_Start) (Variables|Default|GetPortal_End) _新建轨道_0) false false))))

(event EventBeginPlay)

(event Collision|EventActorBeginOverlap
  (params (OtherActor :type Actor%20Object%20Reference)))

(event EventTick
  (params (DeltaSeconds :type Float%20%28single-precision%29)))

(fn ConstructionScript)