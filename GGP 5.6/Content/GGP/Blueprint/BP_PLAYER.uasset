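; Player character Blueprint handling combat, scripted camera blends and hold-to-buy interaction.
; Mouse wheel toggles knife and gun, and left click runs a sphere-trace melee hit on another Identity or a cooldown-limited bullet spawn.
; Holding E at a box drains GameInstance money into UI_press on a looping timer until Levelup, with early release restoring the balance.
; LC events blend the view to SC1–3 and back, while Remake events reapply speed and health.
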(event Custom|Remake%20speed
  (Variables|/Script/Engine.CharacterMovementComponent|SetMaxWalkSpeed (Variables|Character|GetCharacterMovement) (Variables|Default|Getspeed))
  (bind _foundwidgets (Widget|GetAllWidgetsOfClass "/Game/GGP/UI/ui_wst/UI_Player.UI_Player_C" true))
  (Variables|Default|SetUI_Player (Utilities|Array|Get(acopy) _foundwidgets))
  (bind _asbp_instance (Utilities|Casting|CastToBP_Instance (Game|GetGameInstance)))
  (Variables|Default|SetAs%20BP%20Instance _asbp_instance))

(event Custom|Remake%20HP
  (Variables|Default|Sethp (Variables|Default|GetMaxhp)))

(event Custom|LC3END
  (Game|Player|SetViewTargetwithBlend (Game|GetPlayerController 0) self 2.0 "VTBlend_Linear" 0.0 false))

(event Custom|LC1
  (Utilities|FlowControl|Delay 1.0)
  (Game|Player|SetViewTargetwithBlend (Game|GetPlayerController 0) (Variables|Default|GetSC1) 4.0 "VTBlend_Cubic" 0.0 false))

(event Custom|LC1END
  (Game|Player|SetViewTargetwithBlend (Game|GetPlayerController 0) self 3.0 "VTBlend_Linear" 0.0 false))

(event Custom|spend%20money
  (bind _as_bp_instance (Variables|Default|GetAs%20BP%20Instance))
  (if (== (Variables|/Game/GGP/UI/ui_wst/UI_press.UI_press_C|Getneed%20money (Utilities|Array|Get(acopy) (stale Input|KeyboardEvents|E _foundwidgets))) (Variables|/Game/GGP/UI/ui_wst/UI_press.UI_press_C|Getinvest%20monry (Utilities|Array|Get(acopy) (stale Input|KeyboardEvents|E _foundwidgets))))
    (Variables|Default|Setover%20shopping true)
    (Default|Levelup (Variables|Default|GetAs%20BP%20Instance))
    (Utilities|Time|ClearandInvalidateTimerbyHandle (Variables|Default|GetOpenTimerHandle))
    (elif (> (Variables|/Game/GGP/Blueprint/BP_Instance.BP_Instance_C|Getmoney _as_bp_instance) 0.0)
      (Variables|/Game/GGP/UI/ui_wst/UI_press.UI_press_C|Setinvest%20monry (Utilities|Array|Get(acopy) (stale Input|KeyboardEvents|E _foundwidgets)) (+ (Variables|/Game/GGP/UI/ui_wst/UI_press.UI_press_C|Getinvest%20monry (Utilities|Array|Get(acopy) (stale Input|KeyboardEvents|E _foundwidgets))) 1.0))
      (Variables|/Game/GGP/Blueprint/BP_Instance.BP_Instance_C|Setmoney _as_bp_instance (- (Variables|/Game/GGP/Blueprint/BP_Instance.BP_Instance_C|Getmoney _as_bp_instance) 1.0)))))

(event Custom|LC2
  (Utilities|FlowControl|Delay 1.0)
  (Game|Player|SetViewTargetwithBlend (Game|GetPlayerController 0) (Variables|Default|GetSC2) 3.0 "VTBlend_Cubic" 0.0 false))

(event Custom|LC2END
  (Game|Player|SetViewTargetwithBlend (Game|GetPlayerController 0) self 3.0 "VTBlend_Linear" 0.0 false))

(event Custom|LC3
  (Utilities|FlowControl|Delay 1.0)
  (Game|Player|SetViewTargetwithBlend (Game|GetPlayerController 0) (Variables|Default|GetSC3) 3.0 "VTBlend_Cubic" 0.0 false))

(event EventBeginPlay
  (|CallParentFunction)
  (Variables|/Script/Engine.CharacterMovementComponent|SetMaxWalkSpeed (Variables|Character|GetCharacterMovement) (Variables|Default|Getspeed))
  (bind _foundwidgets (Widget|GetAllWidgetsOfClass "/Game/GGP/UI/ui_wst/UI_Player.UI_Player_C" true))
  (Variables|Default|SetUI_Player (Utilities|Array|Get(acopy) _foundwidgets))
  (bind _asbp_instance (Utilities|Casting|CastToBP_Instance (Game|GetGameInstance)))
  (Variables|Default|SetAs%20BP%20Instance _asbp_instance))

(event EventTick
  (params (DeltaSeconds :type Float%20%28single-precision%29))
  (|CallParentFunction DeltaSeconds))

(event Input|MouseEvents|MouseWheelUp
  (params (Key :type Key%20Structure :default "None"))
  (:Pressed
    (Utilities|FlowControl|DoOnce false :!label _label
      (:Completed
        (if (Variables|Default|GetWeapon_state)
          (Variables|Default|SetWeapon_state false)
          (else
            (Variables|Default|SetWeapon_state true)))
        (Default|SwitchImage (Variables|Default|GetUI_Player)))))
  (:Released
    (goto _label Reset)))

(event Input|KeyboardEvents|E
  (params (Key :type Key%20Structure :default "None"))
  (:Pressed
    (if (Variables|Default|Getbox_interaction)
      (bind _foundwidgets (Widget|GetAllWidgetsOfClass "/Game/GGP/UI/ui_wst/UI_press.UI_press_C" true))
      (Default|ShowBar (Utilities|Array|Get(acopy) _foundwidgets))
      (Variables|Default|Setbegin%20shop%20money (Variables|/Game/GGP/Blueprint/BP_Instance.BP_Instance_C|Getmoney (Variables|Default|GetAs%20BP%20Instance)))
      (bind _returnvalue (Utilities|Time|SetTimerbyEvent (delegate Custom|spend%20money) 0.2 true))
      (Variables|Default|SetOpenTimerHandle _returnvalue)))
  (:Released
    (bind _foundwidgets_2 (Widget|GetAllWidgetsOfClass "/Game/GGP/UI/ui_wst/UI_press.UI_press_C" true))
    (if (> (Utilities|Array|Length _foundwidgets_2) 0)
      (Default|HiddenBar (Utilities|Array|Get(acopy) _foundwidgets_2))
      (if (Variables|Default|Getover%20shopping)
        (Variables|/Game/GGP/UI/ui_wst/UI_press.UI_press_C|Setinvest%20monry (Utilities|Array|Get(acopy) _foundwidgets_2) 0.0)
        (else
          (Variables|/Game/GGP/Blueprint/BP_Instance.BP_Instance_C|Setmoney (Variables|Default|GetAs%20BP%20Instance) (Variables|Default|Getbegin%20shop%20money))))
      (Utilities|Time|ClearandInvalidateTimerbyHandle (Variables|Default|GetOpenTimerHandle)))))

(event Input|MouseEvents|MouseWheelDown
  (params (Key :type Key%20Structure :default "None"))
  (:Pressed
    (Utilities|FlowControl|DoOnce false :!label _label
      (:Completed
        (if (Variables|Default|GetWeapon_state)
          (Variables|Default|SetWeapon_state false)
          (else
            (Variables|Default|SetWeapon_state true)))
        (Default|SwitchImage (Variables|Default|GetUI_Player)))))
  (:Released
    (goto _label Reset)))

(event Input|MouseEvents|LeftMouseButton
  (params (Key :type Key%20Structure :default "None"))
  (:Pressed
    (if (Variables|Default|GetWeapon_state)
      (Utilities|PlayerFireKnife)
      (else
        (Utilities|PlayerFireShotting)))))

(fn ConstructionScript)