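; Base character Blueprint providing health, one-time death and a simple area attack.
; BeginPlay fills HP from max, and incoming damage lowers it to zero at most, where a guarded handler calls OnDeath.
; Attack runs a debug-drawn multi-sphere trace around the character, scaled from capsule half-height.
; BP_EnemyBase hits with a different Identity trigger ApplyDamage, though no damaged actor is specified.
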(event Custom|HandleDeath
  ;[0.15 0.15 0.15 0.5] Handle dead
  (if (not (Variables|Default|Getis_dead))
    (Variables|Default|Setis_dead true)
    (Default|CallOnDeath)))

(event Custom|Attack
  (bind _returnvalue (Transformation|GetActorLocation))
  ;[0.15 0.15 0.15 0.5] Simple attack implementation
  (bind _outhits (Collision|MultiSphereTraceByChannel _returnvalue _returnvalue (* (Components|Capsule|GetScaledCapsuleHalfHeight (Variables|Collision|GetCapsuleComponent)) 2.0) "TraceTypeQuery1" false 0 "ForDuration"))
  (for _array_element _outhits
    (bind _asbp_enemy_base (Utilities|Casting|CastToBP_EnemyBase (.HitActor (Collision|BreakHitResult _array_element))))
    (if (Utilities|Enum|NotEqual(Enum) (Variables|BP_CharBase_C|Getidentity _asbp_enemy_base) (Variables|Default|Getidentity))
      (Game|Damage|ApplyDamage 0 (Variables|Default|GetDamage) 0 self))))

(event Custom|DamageHandle
  (params (damage :type Float%20%28double-precision%29))
  ;[0.15 0.15 0.15 0.5] Receive Damage
  (bind _output_get (Variables|Default|SetHP (Math|Float|Max(Float) (- (Variables|Default|GetHP) damage) 0.0)))
  (if (== _output_get 0.0)
    (CallFunction|HandleDeath)))

(event EventBeginPlay
  (Variables|Default|Sethp (Variables|Default|GetMaxhp)))

(event EventTick
  (params (DeltaSeconds :type Float%20%28single-precision%29))
  (|CallParentFunction DeltaSeconds))

(event Game|Damage|EventAnyDamage
  (params (Damage :type Float%20%28single-precision%29) (DamageType :type Damage%20Type%20Object%20Reference) (InstigatedBy :type Controller%20Object%20Reference) (DamageCauser :type Actor%20Object%20Reference))
  ;[0.15 0.15 0.15 0.5] Receive Damage
  (CallFunction|DamageHandle Damage))

(fn ConstructionScript)