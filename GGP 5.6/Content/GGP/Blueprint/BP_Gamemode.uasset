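; Game mode Blueprint that sets up the player HUD and handles closing the upgrade screen.
; On BeginPlay it adds UI_Player to the viewport, then caches BP_Instance and calls its AddCardArry.
; The delatewidge event restores normal time dilation, game-only input and a hidden cursor, then removes the first top-level UI_Player_Upgrade widget found by class search, without an empty check, and prints a debug string.
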(event Custom|delate%20widge
  (bind _returnvalue (Game|GetPlayerController 0))
  (Utilities|Time|SetGlobalTimeDilation 1.0)
  (Input|SetInputModeGameOnly _returnvalue false)
  (Variables|/Script/Engine.PlayerController|SetbShowMouseCursor _returnvalue false)
  (bind _foundwidgets (Widget|GetAllWidgetsOfClass "/Game/GGP/UI/ui_wst/UI_Player_Upgrade.UI_Player_Upgrade_C" true))
  (Widget|RemovefromParent (Utilities|Array|Get(acopy) _foundwidgets))
  (Development|PrintString "Hello"))

(event EventBeginPlay
  (Utilities|FlowControl|Sequence
    (:then_0
      (bind _returnvalue (UserInterface|CreateWidget "/Game/GGP/UI/ui_wst/UI_Player.UI_Player_C"))
      (UserInterface|Viewport|AddtoViewport _returnvalue 0)
      (bind _asbp_instance (Utilities|Casting|CastToBP_Instance (Game|GetGameInstance)))
      (bind _output_get (Variables|Default|SetAs%20BP%20Instance _asbp_instance))
      (Default|AddCardArry _output_get))))

(event EventTick
  (params (DeltaSeconds :type Float%20%28single-precision%29)))

(fn ConstructionScript)