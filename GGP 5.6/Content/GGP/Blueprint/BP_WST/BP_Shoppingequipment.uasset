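; BP_Shoppingequipment is an equipment shop trigger actor that sells the player access to an upgrade screen.
; When BP_PLAYER overlaps its Box, it checks Money on the BP_Instance game instance and deducts a fixed price if affordable.
; It then opens UI_Player_Upgrade and switches to UI-only input focused on that widget.
; The charge happens on entry, before any upgrade is chosen, and insufficient money produces no response.
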(event OnComponentBeginOverlap(Box)
  (params (OverlappedComponent :type Primitive%20Component%20Object%20Reference) (OtherActor :type Actor%20Object%20Reference) (OtherComp :type Primitive%20Component%20Object%20Reference) (OtherBodyIndex :type Integer) (bFromSweep :type Boolean) (SweepResult :type Hit%20Result%20Structure%20%28by%20ref%29))
  (Utilities|Casting|CastToBP_PLAYER OtherActor)
  (bind _asbp_instance (Utilities|Casting|CastToBP_Instance (Game|GetGameInstance)))
  (Variables|Default|SetAs%20BP%20Instance _asbp_instance)
  (if (>= (Variables|/Game/GGP/Blueprint/BP_Instance.BP_Instance_C|Getmoney _asbp_instance) 1e+02)
    (Variables|/Game/GGP/Blueprint/BP_Instance.BP_Instance_C|Setmoney (Variables|Default|GetAs%20BP%20Instance) (- (Variables|/Game/GGP/Blueprint/BP_Instance.BP_Instance_C|Getmoney (Variables|Default|GetAs%20BP%20Instance)) 1e+02))
    (bind _returnvalue (UserInterface|CreateWidget "/Game/GGP/UI/ui_wst/UI_Player_Upgrade.UI_Player_Upgrade_C"))
    (UserInterface|Viewport|AddtoViewport _returnvalue 0)
    (Input|SetInputModeUIOnly (Game|GetPlayerController 0) _returnvalue "DoNotLock" false)))

(event EventBeginPlay)

(event Collision|EventActorBeginOverlap
  (params (OtherActor :type Actor%20Object%20Reference)))

(event EventTick
  (params (DeltaSeconds :type Float%20%28single-precision%29)))

(fn ConstructionScript)