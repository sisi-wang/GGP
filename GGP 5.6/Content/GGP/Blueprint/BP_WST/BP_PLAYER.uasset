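; BP_PLAYER is the player character Blueprint, holding speed and health resets plus scripted camera transitions.
; BeginPlay and Remakespeed apply Speed to the movement component's max walk speed, while RemakeHP restores Hp to Maxhp.
; LC1 to LC3 wait briefly, then cubic-blend the view to targets SC1 to SC3.
; Their matching END events blend the view back to the player.
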(event Custom|Remake%20speed
  (Variables|/Script/Engine.CharacterMovementComponent|SetMaxWalkSpeed (Variables|Character|GetCharacterMovement) (Variables|Default|Getspeed)))

(event Custom|Remake%20HP
  (Variables|Default|Sethp (Variables|Default|GetMaxhp)))

(event Custom|LC3END
  (Game|Player|SetViewTargetwithBlend (Game|GetPlayerController 0) self 2.0 "VTBlend_Linear" 0.0 false))

(event Custom|LC1
  (Utilities|FlowControl|Delay 1.0)
  (Game|Player|SetViewTargetwithBlend (Game|GetPlayerController 0) (Variables|Default|GetSC1) 4.0 "VTBlend_Cubic" 0.0 false))

(event Custom|LC1END
  (Game|Player|SetViewTargetwithBlend (Game|GetPlayerController 0) self 3.0 "VTBlend_Linear" 0.0 false))

(event Custom|LC2
  (Utilities|FlowControl|Delay 1.0)
  (Game|Player|SetViewTargetwithBlend (Game|GetPlayerController 0) (Variables|Default|GetSC2) 3.0 "VTBlend_Cubic" 0.0 false))

(event Custom|LC2END
  (Game|Player|SetViewTargetwithBlend (Game|GetPlayerController 0) self 3.0 "VTBlend_Linear" 0.0 false))

(event Custom|LC3
  (Utilities|FlowControl|Delay 1.0)
  (Game|Player|SetViewTargetwithBlend (Game|GetPlayerController 0) (Variables|Default|GetSC3) 3.0 "VTBlend_Cubic" 0.0 false))

(event EventBeginPlay
  (|CallParentFunction)
  (Variables|/Script/Engine.CharacterMovementComponent|SetMaxWalkSpeed (Variables|Character|GetCharacterMovement) (Variables|Default|Getspeed)))

(event EventTick
  (params (DeltaSeconds :type Float%20%28single-precision%29))
  (|CallParentFunction DeltaSeconds))

(fn ConstructionScript)