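; Projectile bullet that damages enemies on overlap and destroys itself three seconds after spawning if it has not already hit one.
; BeginPlay copies Speed into the projectile movement's max and initial speed, then starts the lifetime delay.
; Sphere overlap applies BaseDamage to BP_EnemyBase actors and destroys the bullet.
; Other actors receive OnBulletHitMessage with the bullet as argument, and the bullet is not destroyed here.
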(event OnComponentBeginOverlap(Sphere1)
  (params (OverlappedComponent :type Primitive%20Component%20Object%20Reference) (OtherActor :type Actor%20Object%20Reference) (OtherComp :type Primitive%20Component%20Object%20Reference) (OtherBodyIndex :type Integer) (bFromSweep :type Boolean) (SweepResult :type Hit%20Result%20Structure%20%28by%20ref%29))
  (bind _asbp_enemy_base (Utilities|Casting|CastToBP_EnemyBase OtherActor)
    (:then
      (Game|Damage|ApplyDamage _asbp_enemy_base (Variables|Default|GetBase%20Damage) 0 0)
      (Actor|DestroyActor))
    (:CastFailed
      (Class|BPIBulletInteraction|OnBulletHit(Message) OtherActor self))))

(event EventBeginPlay
  (bind _projectilemovement (Variables|Default|GetProjectileMovement))
  (bind _output_get (Variables|/Script/Engine.ProjectileMovementComponent|SetMaxSpeed _projectilemovement (Variables|Default|Getspeed)))
  (Variables|/Script/Engine.ProjectileMovementComponent|SetInitialSpeed _projectilemovement _output_get)
  (Utilities|FlowControl|Delay 3.0)
  (Actor|DestroyActor))

(event Collision|EventActorBeginOverlap
  (params (OtherActor :type Actor%20Object%20Reference)))

(event EventTick
  (params (DeltaSeconds :type Float%20%28single-precision%29)))

(fn ConstructionScript)