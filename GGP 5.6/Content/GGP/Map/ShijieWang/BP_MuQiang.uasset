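; BP_MuQiang is a breakable wooden wall actor that the player can destroy up close.
; A Box overlap with BP_PLAYER toggles the IsTouchingPlayer flag on entry and exit.
; A left mouse press handled inside the actor checks that flag, then plays the board-breaking sound at the wall's location and destroys the actor.
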(event OnComponentBeginOverlap(Box)
  (params (OverlappedComponent :type Primitive%20Component%20Object%20Reference) (OtherActor :type Actor%20Object%20Reference) (OtherComp :type Primitive%20Component%20Object%20Reference) (OtherBodyIndex :type Integer) (bFromSweep :type Boolean) (SweepResult :type Hit%20Result%20Structure%20%28by%20ref%29))
  (Utilities|Casting|CastToBP_PLAYER OtherActor)
  (Variables|Default|SetIsTouchingPlayer true))

(event OnComponentEndOverlap(Box)
  (params (OverlappedComponent :type Primitive%20Component%20Object%20Reference) (OtherActor :type Actor%20Object%20Reference) (OtherComp :type Primitive%20Component%20Object%20Reference) (OtherBodyIndex :type Integer))
  (Utilities|Casting|CastToBP_PLAYER OtherActor)
  (Variables|Default|SetIsTouchingPlayer false))

(event EventBeginPlay)

(event EventTick
  (params (DeltaSeconds :type Float%20%28single-precision%29)))

(event Input|MouseEvents|LeftMouseButton
  (params (Key :type Key%20Structure :default "None"))
  (:Pressed
    (if (Variables|Default|GetIsTouchingPlayer)
      (Audio|SpawnSoundatLocation "/Game/GGP/Map/ShijieWang/AudioEffects/AE_Mubanduanlie.AE_Mubanduanlie" (Transformation|GetActorLocation) "0, 0, 0" 1.0 1.0 0.0 0 0)
      (Actor|DestroyActor))))

(fn ConstructionScript)